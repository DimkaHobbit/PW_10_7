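; BP_VerySmartSphere is a practice pawn that endlessly wanders to random points around its spawn location.
; MoveToTarget picks a point in a flat box centered on the start location, runs AI MoveTo, and calls itself again on success or failure.
; Movement speed feeds FloatingPawnMovement at BeginPlay, and Tick draws a debug sphere above the current target.
; GenerateNewTargetPoint is an empty stub.
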(event Custom|MoveToTarget
  (Variables|Default|SetTargetLocation (Math|Random|RandomPointinBoundingBox (Variables|Default|GetStartLocation) "500.000000,500.000000,0.000000"))
  (bind _movementresult (AI|AIMoveTo self (Variables|Default|GetTargetLocation) 0 1e+01 true)
    (:then
      (Development|PrintString (Utilities|String|EnumtoString _movementresult) true true "(R=0.000000,G=0.660000,B=1.000000,A=1.000000)" 1.0))
    (:OnSuccess
      (CallFunction|MovetoTarget :!label _label))
    (:OnFail
      (goto _label))))

(event EventBeginPlay
  (Variables|Default|SetStartLocation (Transformation|GetActorLocation))
  (Variables|/Script/Engine.FloatingPawnMovement|SetMaxSpeed (Variables|Default|GetFloatingPawnMovement) (Variables|Default|GetSpeed))
  (CallFunction|MovetoTarget))

(event EventTick
  (params (DeltaSeconds :type Float%20%28single-precision%29))
  (bind _targetlocation (Variables|Default|GetTargetLocation))
  (bind (_x _y _z) (Class|KismetMathLibrary|BreakVector3f _targetlocation))
  (Rendering|Debug|DrawDebugSphere (Math|Vector|MakeVector _x _y (+ _z 1e+02)) 3e+01 12 "(R=0.000000,G=0.098334,B=1.000000,A=1.000000)" 0.0))

(fn ConstructionScript)

(fn GenerateNewTargetPoint)